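; BP_SpawnUI shows story dialogue through a WBP_Story user widget held by its Widget.
; On BeginPlay it casts and caches that widget, sets PlayerViewing to true, and calls ContinueDialogue.
; ContinueDialogue sends Dialogue to the widget while PlayerViewing is true and hides it otherwise.
; A constant true branch means AdvanceDialogue is never reached, and the widget's DialogueComplete is unused.
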(event `self.ReceiveBeginPlay`
  (bind _aswbp_story (cast `/Game/Blueprints/WBP_Story` (`WidgetComponent.GetUserWidgetObject` (`self.Widget`))))
  (set `self.As WBP Story` _aswbp_story)
  (set `self.PlayerViewing` true)
  (`self.ContinueDialogue`))

(event `ContinueDialogue`
  (bind _as_wbp_story (`self.As WBP Story`))
  (if (`self.PlayerViewing`)
    (if true
      (`/Game/Blueprints/WBP_Story.SetDialogue` _as_wbp_story (`self.Dialogue`))
      (else
        (`/Game/Blueprints/WBP_Story.AdvanceDialogue` _as_wbp_story)))
    (else
      (`/Game/Blueprints/WBP_Story.HideDialogue` (`self.As WBP Story`)))))

(fn `UserConstructionScript`)